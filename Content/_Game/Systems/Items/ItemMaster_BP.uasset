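; Base item Blueprint that the player picks up into a hand grip and drops back to its original placement.
; Interactwith registers it as the controller's CurrentItem, disables collision, attaches it to ItemGrip and timeline-lerps it there.
; EDrop detaches it, lerps it to the transform cached in the Construction Script, then restores collision.
; IsMoving blocks both events mid-animation; a separate DropItem function only applies a zero-alpha lerp, without a timeline.
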(event `/Game/_Game/Blueprint/Core/I_Interact_BP.InteractWith`
  (params (PlayerController :type "/Game/_Game/Blueprint/Character/PlayerController_BP Object Reference"))
  (bind _itemgrip (`/Game/_Game/Blueprint/Character/PlayerCharacter_BP.ItemGrip` (`/Game/_Game/Blueprint/Character/PlayerController_BP.PlayerRef` (`self.ControllerRef`))))
  (if (not (`self.bIsMoving`))
    (set `self.bIsMoving` true)
    (set `self.bIsEnabled` false)
    (bind _output_get (set `self.ControllerRef` PlayerController))
    (set `/Game/_Game/Blueprint/Character/PlayerController_BP.CurrentItem` self _output_get)
    (`PrimitiveComponent.SetCollisionEnabled` (`self.StaticMesh`) "NoCollision")
    (`|ExecutionSequence`
      (:`then_0`
        (bind (_direction _percent) (`Timeline|Timeline` :!via `PlayFromStart`)
          (:`Update`
            (`self.K2_SetActorLocationAndRotation` (`KismetMathLibrary.VLerp` (`self.K2_GetActorLocation`) (`SceneComponent.K2_GetComponentLocation` _itemgrip) _percent) (`KismetMathLibrary.RLerp` (`self.K2_GetActorRotation`) (`SceneComponent.K2_GetComponentRotation` _itemgrip) _percent true)))
          (:`Finished`
            (set `self.bIsMoving` false)
            (set `self.bIsEnabled` true))))
      (:`then_1`
        (`self.K2_AttachToComponent` (`/Game/_Game/Blueprint/Character/PlayerCharacter_BP.ItemGrip` (`/Game/_Game/Blueprint/Character/PlayerController_BP.PlayerRef` (`self.ControllerRef`))) "None" "KeepWorld" "KeepWorld" "KeepRelative")))))

(event `EDrop`
  (params (ControllerRef :type "/Game/_Game/Blueprint/Character/PlayerController_BP Object Reference"))
  (bind (_initialtransform_location _initialtransform_rotation) (`KismetMathLibrary.BreakTransform` (`self.InitialTransform`)))
  (if (not (`self.bIsMoving`))
    (set `self.ControllerRef` ControllerRef)
    (set `self.bIsEnabled` false)
    (`self.K2_DetachFromActor` (`/Game/_Game/Blueprint/Character/PlayerController_BP.CurrentItem` (`self.ControllerRef`)) "KeepWorld" "KeepWorld" "KeepRelative")
    (set `self.bIsMoving` true)
    (set `/Game/_Game/Blueprint/Character/PlayerController_BP.CurrentItem` null (`self.ControllerRef`))
    (bind (_direction _percent) (`Timeline|Timeline_0` :!via `PlayFromStart`)
      (:`Update`
        (`self.K2_SetActorLocationAndRotation` (`KismetMathLibrary.VLerp` (`self.K2_GetActorLocation`) _initialtransform_location _percent) (`KismetMathLibrary.RLerp` (`self.K2_GetActorRotation`) _initialtransform_rotation _percent true)))
      (:`Finished`
        (set `self.bIsMoving` false)
        (`PrimitiveComponent.SetCollisionEnabled` (`self.StaticMesh`) "QueryAndPhysics")
        (set `self.bIsEnabled` true)))))

(fn `DropItem`
  (params (ControllerRef :type "/Game/_Game/Blueprint/Character/PlayerController_BP Object Reference"))
  (bind (_initialtransform_location _initialtransform_rotation) (`KismetMathLibrary.BreakTransform` (`self.InitialTransform`)))
  (if (`self.bIsMoving`)
    (bind _output_get (set `self.ControllerRef` ControllerRef))
    (set `/Game/_Game/Blueprint/Character/PlayerController_BP.CurrentItem` self _output_get)
    (set `self.bIsMoving` true)
    (`self.K2_SetActorLocationAndRotation` (`KismetMathLibrary.VLerp` (`self.K2_GetActorLocation`) _initialtransform_location) (`KismetMathLibrary.RLerp` (`self.K2_GetActorRotation`) _initialtransform_rotation 0.0 true))))

(fn `UserConstructionScript`
  (`parent.UserConstructionScript`)
  (set `self.InitialTransform` (`KismetMathLibrary.MakeTransform` (`self.K2_GetActorLocation`) (`self.K2_GetActorRotation`))))
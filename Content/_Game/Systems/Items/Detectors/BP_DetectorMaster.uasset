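; BP_DetectorMaster is a base detector item that reacts to specific NPC classes entering its sphere.
; While enabled and not already reacting, an overlapping NPC_Master whose exact class is in FItemStruct.CreaturesReact triggers React.
; Any NPC_Master leaving the sphere during a reaction triggers StopReact, without checking that list.
; Both functions only print debug text and toggle IsInteracted, which Tick prints every frame.
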(event `self.ReceiveTick`
  (params (DeltaSeconds :type "Float (single-precision)"))
  (`KismetSystemLibrary.PrintString` (`KismetStringLibrary.Conv_BoolToString` (`self.bIsInteracted`)) true true (struct :`G` 0.66 :`B` 1.0 :`A` 1.0) DeltaSeconds))

(event `self.Sphere.OnComponentBeginOverlap`
  (params (OverlappedComponent :type "PrimitiveComponent Object Reference") (OtherActor :type "Actor Object Reference") (OtherComp :type "PrimitiveComponent Object Reference") (OtherBodyIndex :type Integer) (bFromSweep :type Boolean) (SweepResult :type "HitResult Structure (by ref)"))
  (if (`self.bIsEnabled`)
    (if (not (`self.bIsInteracted`))
      (bind _asnpc_master (cast `/Game/_Game/Blueprint/NPC/NPC_Master` OtherActor))
      (for _array_element (`.CreaturesReact_22_E0081E854B79AFEA3AB2C1A583AE1F65` (break `/Game/_Game/Systems/Items/Misc/FItemStruct` (`self.FItemStruct`)))
        (bind _returnvalue (`GameplayStatics.GetObjectClass` _asnpc_master))
        (if (== _array_element _returnvalue)
          (`|ExecutionSequence`
            (:`then_0`
              (`self.React` _returnvalue))
            (:`then_1`
              (break))))))))

(event `self.Sphere.OnComponentEndOverlap`
  (params (OverlappedComponent :type "PrimitiveComponent Object Reference") (OtherActor :type "Actor Object Reference") (OtherComp :type "PrimitiveComponent Object Reference") (OtherBodyIndex :type Integer))
  (if (`self.bIsInteracted`)
    (bind _asnpc_master (cast `/Game/_Game/Blueprint/NPC/NPC_Master` OtherActor))
    (`self.StopReact` (`GameplayStatics.GetObjectClass` _asnpc_master))))

(fn `React`
  (params (NPC_Class :type "/Game/_Game/Blueprint/NPC/NPC_Master Class Reference"))
  (`KismetSystemLibrary.PrintString` (`KismetStringLibrary.Concat_StrStr` (`KismetStringLibrary.Concat_StrStr` (`KismetSystemLibrary.GetClassDisplayName` (`GameplayStatics.GetObjectClass` self)) "React to") (`KismetSystemLibrary.GetClassDisplayName` NPC_Class)) true true (struct :`R` 0.001175 :`G` 1.0 :`A` 1.0))
  (set `self.bIsInteracted` true))

(fn `StopReact`
  (params (NPC_Class :type "/Game/_Game/Blueprint/NPC/NPC_Master Class Reference"))
  (`KismetSystemLibrary.PrintString` (`KismetStringLibrary.Concat_StrStr` (`KismetStringLibrary.Concat_StrStr` (`KismetSystemLibrary.GetClassDisplayName` (`GameplayStatics.GetObjectClass` self)) "Stop react to") (`KismetSystemLibrary.GetClassDisplayName` NPC_Class)) true true (struct :`R` 1.0 :`B` 0.063817 :`A` 1.0))
  (set `self.bIsInteracted` false))

(fn `UserConstructionScript`
  (`parent.UserConstructionScript`))
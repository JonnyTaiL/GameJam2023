(event `self.ReceiveBeginPlay`)

(fn `Add score`
  (params (Amount :type "Float (double-precision)"))
  (bind _output_get (set `self.Score` (+ (`self.Score`) Amount)))
  (`/Game/_Game/Blueprint/UI/UI_Main.UpdateScore` (`self.WidgetRef`) _output_get))

(fn `Subtract Score`
  (params (Amount :type "Float (double-precision)"))
  (bind _returnvalue (- (`self.Score`) Amount))
  (if (>= _returnvalue 0.0)
    (bind _output_get (set `self.Score` _returnvalue))
    (`/Game/_Game/Blueprint/UI/UI_Main.UpdateScore` (`self.WidgetRef`) _output_get)
    (else
      (bind _output_get_2 (set `self.Score` 0.0))
      (`/Game/_Game/Blueprint/UI/UI_Main.UpdateScore` (`self.WidgetRef`) _output_get_2))))

(fn `UserConstructionScript`)
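; Door actor that swings open and closed when its Interactwith event fires.
; The DoorSlide timeline drives the yaw of the SMDoor mesh, playing from the start to open and reversing from the end to close.
; A CanInteract flag blocks input during the motion, and the timeline direction sets the Closed state when it finishes.
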(event `/Game/_Game/Blueprint/Core/I_Interact.InteractWith`
  (params (PlayerController :type "/Game/_Game/Blueprint/Character/PlayerController_BP Object Reference"))
  (if (`self.CanInteract`)
    (if (`self.Closed`)
      (set `self.CanInteract` false)
      (bind (_direction _rotate) (`Timeline|DoorSlide` :!via `PlayFromStart` :!label _label)
        (:`Update`
          (`SceneComponent.K2_SetRelativeRotation` (`self.SM_Door`) (`KismetMathLibrary.MakeRotator` 0.0 0.0 _rotate) false false))
        (:`Finished`
          (set `self.CanInteract` true)
          (switch `ETimelineDirection` _direction
            (:`Forward`
              (set `self.Closed` false))
            (:`Backward`
              (set `self.Closed` true)))))
      (else
        (set `self.CanInteract` false)
        (goto _label :!via `ReverseFromEnd`)))))

(fn `UserConstructionScript`)
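; Radio_BP is an interactable environment radio that toggles its audio on and off.
; On BeginPlay the PlayAtStart flag decides whether the Audio component starts paused or playing, tracked in a Playing variable.
; Interacting pauses or resumes the audio rather than restarting it.
; Look-at events toggle custom depth on the StaticMesh, and interacting also enables it.
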(event `self.ReceiveBeginPlay`
  (bind _audio (`self.Audio`))
  (if (`self.PlayAtStart`)
    (`AudioComponent.SetPaused` _audio false)
    (else
      (`AudioComponent.SetPaused` _audio true)))
  (set `self.Playing` (`self.PlayAtStart`)))

(event `/Game/_Game/Blueprint/Core/I_Interact_BP.InteractWith`
  (params (PlayerController :type "/Game/_Game/Blueprint/Character/PlayerController_BP Object Reference"))
  (bind _audio (`self.Audio`))
  (if (`self.Playing`)
    (`AudioComponent.SetPaused` _audio true)
    (set `self.Playing` false)
    (else
      (`AudioComponent.SetPaused` _audio false)
      (set `self.Playing` true)))
  (`PrimitiveComponent.SetRenderCustomDepth` (`self.StaticMesh`) true))

(event `/Game/_Game/Blueprint/Core/I_Interact_BP.LookAt`
  (params (PlayerController :type "/Game/_Game/Blueprint/Character/PlayerController_BP Object Reference"))
  (`PrimitiveComponent.SetRenderCustomDepth` (`self.StaticMesh`) true))

(event `/Game/_Game/Blueprint/Core/I_Interact_BP.StopLookAt`
  (params (PlayerController :type "/Game/_Game/Blueprint/Character/PlayerController_BP Object Reference"))
  (`PrimitiveComponent.SetRenderCustomDepth` (`self.StaticMesh`) false))

(fn `UserConstructionScript`)
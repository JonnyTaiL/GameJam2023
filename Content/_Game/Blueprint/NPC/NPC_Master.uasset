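; Base NPC visitor that knocks at a door and awaits a treat or repellent from the player.
; Construction picks a random child mesh, whose index selects animations, voice lines and eye material slot.
; Interaction scores the item against human or monster type; exact repellents trigger particles and, where supported, glowing eyes, then the NPC leaves and restarts its spawner countdown.
; Sphere overlaps drive item reaction messages; the CheckItems polling timer is unwired.
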(event `CheckItems`
  (bind _charinfo_idname (break `/Game/_Game/Blueprint/NPC/FCreatureStruct` (`self.CharInfo`)))
  (for _array_element (`self.GetOverlappingActors` "/Game/_Game/Blueprint/Items/ItemMaster_BP.ItemMaster_BP_C")
    (bind _asitem_master_bp (cast `/Game/_Game/Blueprint/Items/ItemMaster_BP` _array_element)
      (:`then`
        (bind _output_get (set `self.ItemRef` _asitem_master_bp))
        (message `/Game/_Game/Blueprint/Core/I_Reaction.React` _output_get _charinfo_idname)
        (break))
      (:`CastFailed`
        (`self.ItemRef`
          (:`then`
            (message `/Game/_Game/Blueprint/Core/I_Reaction.StopReact` (`self.ItemRef`) _charinfo_idname))
          (:`else`))))))

(event `self.Sphere.OnComponentBeginOverlap`
  (params (OverlappedComponent :type "PrimitiveComponent Object Reference") (OtherActor :type "Actor Object Reference") (OtherComp :type "PrimitiveComponent Object Reference") (OtherBodyIndex :type Integer) (bFromSweep :type Boolean) (SweepResult :type "HitResult Structure (by ref)"))
  (bind _charinfo_idname (break `/Game/_Game/Blueprint/NPC/FCreatureStruct` (`self.CharInfo`)))
  (if (`KismetSystemLibrary.DoesImplementInterface` OtherActor "/Game/_Game/Blueprint/Core/I_Reaction.I_Reaction_C")
    (message `/Game/_Game/Blueprint/Core/I_Reaction.React` OtherActor _charinfo_idname)))

(event `self.Sphere.OnComponentEndOverlap`
  (params (OverlappedComponent :type "PrimitiveComponent Object Reference") (OtherActor :type "Actor Object Reference") (OtherComp :type "PrimitiveComponent Object Reference") (OtherBodyIndex :type Integer))
  (bind _charinfo_idname (break `/Game/_Game/Blueprint/NPC/FCreatureStruct` (`self.CharInfo`)))
  (if (`KismetSystemLibrary.DoesImplementInterface` OtherActor "/Game/_Game/Blueprint/Core/I_Reaction.I_Reaction_C")
    (message `/Game/_Game/Blueprint/Core/I_Reaction.StopReact` OtherActor _charinfo_idname)))

(event `OnDestroyed_Event` :!signature `self.OnDestroyed`
  (params (DestroyedActor :type "Actor Object Reference"))
  (`/Game/_Game/Blueprint/NPC/Npc_Spawner_BP.StartCount` (`self.SpawnerRef`)))

(event `self.ReceiveBeginPlay`
  (`|ExecutionSequence`
    (:`then_0`
      (`self.SpawnParticles`)
      (bind _asgs_share_your_treat (cast `/Game/_Game/Blueprint/Core/GS_ShareYourTreat` (`GameplayStatics.GetGameState`))
        (:`then`
          (set `self.GameStateRef` _asgs_share_your_treat)
          (add `self.OnDestroyed` (delegate `OnDestroyed_Event`)))
        (:`CastFailed`
          (`KismetSystemLibrary.PrintString` "NO GAME STATE"))))
    (:`then_1`
      ;[1 1 1] Door knock
      (`/Game/_Game/Blueprint/Environment/Door_BP.PlayKnockSound` (`self.DoorRef`))
      (`SkeletalMeshComponent.PlayAnimation` (`self.Mesh`) (`|GetArrayItem` (`self.Montages`) (select `int` (`self.AnimIndex`) :`0` 0 :`1` 3 :`2` 6 :`3` 9 :`4` 12)) true)
      (`KismetSystemLibrary.Delay` 0.2)
      (set `/Game/_Game/Blueprint/Environment/Door_BP.CanInteract` true (`self.DoorRef`))
      (`/Game/_Game/Blueprint/Environment/Door_BP.StartRepeatCount` (`self.DoorRef`)))
    (:`then_2`
      (if (>= (select `int` (`self.AnimIndex`) :`0` -1 :`1` 5 :`2` 7 :`3` 4 :`4` 3) 0)
        (bind _returnvalue (`KismetMaterialLibrary.CreateDynamicMaterialInstance` "/Game/_Assets/Meshes/Boy3/Skins/M_Eyes.M_Eyes"))
        (set `self.EyesMaterial` _returnvalue)
        (bind _doorref (`self.DoorRef`)
          (:`then`
            (set `/Game/_Game/Blueprint/Environment/Door_BP.NPCRef` self _doorref)
            (bind _returnvalue_2 (`KismetSystemLibrary.K2_SetTimerDelegate` (delegate `TimeVoice`) 15.0 true))
            (set `self.VoiceHandle` _returnvalue_2))
          (:`else`))))))

(event `TimeVoice`
  (`self.PlayVoiceline` "NewEnumerator3"))

(event `/Game/_Game/Blueprint/Core/I_Interact.InteractWith`
  (params (PlayerController :type "/Game/_Game/Blueprint/Character/PlayerController_BP Object Reference"))
  (bind (_charinfo_idname _charinfo_ismonster _charinfo_enemytype _charinfo_types) (break `/Game/_Game/Blueprint/NPC/FCreatureStruct` (`self.CharInfo`)))
  (bind _mesh (`self.Mesh`))
  (bind _gamestateref (`self.GameStateRef`))
  ;[1 1 1] ClusterFuck
  (if (not (`self.Interacted`))
    (bind _currentitem (`/Game/_Game/Blueprint/Character/PlayerController_BP.CurrentItem` PlayerController)
      (:`then`
        (set `self.Interacted` true)
        (switch `/Game/_Game/Blueprint/NPC/E_NPCTypes` _charinfo_types
          (:`NewEnumerator0`
            (bind (_iteminfo_idname _iteminfo_itemtype _iteminfo_monstersreact _iteminfo_eitem) (break `/Game/_Game/Blueprint/Items/FItemStruct` (`/Game/_Game/Blueprint/Items/ItemMaster_BP.ItemInfo` _currentitem)))
            (switch `/Game/_Game/Blueprint/Items/EItems` _iteminfo_eitem
              (:`NewEnumerator0`
                (`self.PlayVoiceline` "NewEnumerator2" :!label _label)
                (`/Game/_Game/Blueprint/Core/GS_ShareYourTreat.Subtract Score` _gamestateref 500.0)
                (`SkeletalMeshComponent.PlayAnimation` _mesh (`|GetArrayItem` (`self.Montages`) (select `int` (`self.AnimIndex`) :`0` 1 :`1` 4 :`2` 7 :`3` 10 :`4` 13)) false)
                (`KismetSystemLibrary.Delay` 2.0)
                (`/Game/_Game/Blueprint/Environment/Door_BP.CloseDoor` (`self.DoorRef`))
                (`KismetSystemLibrary.Delay` 1.0)
                (`self.K2_DestroyActor`))
              (:`NewEnumerator7`
                (goto _label))
              (:`NewEnumerator8`
                (goto _label))
              (:`NewEnumerator9`
                (goto _label))
              (:`NewEnumerator1`
                (`self.PlayVoiceline` "NewEnumerator1")
                (`/Game/_Game/Blueprint/Core/GS_ShareYourTreat.Add score` _gamestateref 500.0)
                (`SkeletalMeshComponent.PlayAnimation` _mesh (`|GetArrayItem` (`self.Montages`) (select `int` (`self.AnimIndex`) :`0` 2 :`1` 5 :`2` 8 :`3` 11 :`4` 14)) false)
                (`KismetSystemLibrary.Delay` 5.5)
                (`/Game/_Game/Blueprint/Environment/Door_BP.CloseDoor` (`self.DoorRef`))
                (`KismetSystemLibrary.Delay` 1.0)
                (`self.K2_DestroyActor`))))
          (:`NewEnumerator1`
            (switch `/Game/_Game/Blueprint/Items/EItems` _iteminfo_eitem
              (:`NewEnumerator0`
                (if (>= (select `int` (`self.AnimIndex`) :`0` -1 :`1` 5 :`2` 7 :`3` 4 :`4` 3) 0)
                  (`self.SetEyesValues`))
                (`self.FireParticles`)
                (`/Game/_Game/Blueprint/Core/GS_ShareYourTreat.Add score` (`self.GameStateRef`) 500.0)
                (`self.PlayVoiceline` "NewEnumerator2" :!label _label_2)
                (`SkeletalMeshComponent.PlayAnimation` (`self.Mesh`) (`|GetArrayItem` (`self.Montages`) (select `int` (`self.AnimIndex`) :`0` 1 :`1` 4 :`2` 7 :`3` 10 :`4` 13)) false)
                (`KismetSystemLibrary.Delay` 2.0)
                (`/Game/_Game/Blueprint/Environment/Door_BP.CloseDoor` (`self.DoorRef`))
                (`KismetSystemLibrary.Delay` 1.0)
                (`self.K2_DestroyActor`))
              (:`NewEnumerator7`
                (`/Game/_Game/Blueprint/Core/GS_ShareYourTreat.Add score` (`self.GameStateRef`) 100.0 :!label _label_3)
                (goto _label_2))
              (:`NewEnumerator8`
                (goto _label_3))
              (:`NewEnumerator9`
                (goto _label_3))
              (:`NewEnumerator1`
                (`/Game/_Game/Blueprint/Core/GS_ShareYourTreat.Subtract Score` (`self.GameStateRef`) 500.0)
                (`self.PlayVoiceline` "NewEnumerator1")
                (`SkeletalMeshComponent.PlayAnimation` (`self.Mesh`) (`|GetArrayItem` (`self.Montages`) (select `int` (`self.AnimIndex`) :`0` 2 :`1` 5 :`2` 8 :`3` 11 :`4` 14)) false)
                (`KismetSystemLibrary.Delay` 5.5)
                (`/Game/_Game/Blueprint/Environment/Door_BP.CloseDoor` (`self.DoorRef`))
                (`KismetSystemLibrary.Delay` 1.0)
                (`self.K2_DestroyActor`))))
          (:`NewEnumerator2`
            (switch `/Game/_Game/Blueprint/Items/EItems` _iteminfo_eitem
              (:`NewEnumerator0`
                (`/Game/_Game/Blueprint/Core/GS_ShareYourTreat.Add score` (`self.GameStateRef`) 100.0 :!label _label_4)
                (`self.PlayVoiceline` "NewEnumerator2" :!label _label_5)
                (`SkeletalMeshComponent.PlayAnimation` (`self.Mesh`) (`|GetArrayItem` (`self.Montages`) (select `int` (`self.AnimIndex`) :`0` 1 :`1` 4 :`2` 7 :`3` 10 :`4` 13)) false)
                (`KismetSystemLibrary.Delay` 2.0)
                (`/Game/_Game/Blueprint/Environment/Door_BP.CloseDoor` (`self.DoorRef`))
                (`KismetSystemLibrary.Delay` 1.0)
                (`self.K2_DestroyActor`))
              (:`NewEnumerator7`
                (if (>= (select `int` (`self.AnimIndex`) :`0` -1 :`1` 5 :`2` 7 :`3` 4 :`4` 3) 0)
                  (`self.SetEyesValues`))
                (`self.FireParticles`)
                (`/Game/_Game/Blueprint/Core/GS_ShareYourTreat.Add score` (`self.GameStateRef`) 500.0)
                (goto _label_5))
              (:`NewEnumerator8`
                (goto _label_4))
              (:`NewEnumerator9`
                (goto _label_4))
              (:`NewEnumerator1`
                (`/Game/_Game/Blueprint/Core/GS_ShareYourTreat.Subtract Score` (`self.GameStateRef`) 500.0)
                (`self.PlayVoiceline` "NewEnumerator1")
                (`SkeletalMeshComponent.PlayAnimation` (`self.Mesh`) (`|GetArrayItem` (`self.Montages`) (select `int` (`self.AnimIndex`) :`0` 2 :`1` 5 :`2` 8 :`3` 11 :`4` 14)) false)
                (`KismetSystemLibrary.Delay` 5.5)
                (`/Game/_Game/Blueprint/Environment/Door_BP.CloseDoor` (`self.DoorRef`))
                (`KismetSystemLibrary.Delay` 1.0)
                (`self.K2_DestroyActor`))))
          (:`NewEnumerator3`
            (switch `/Game/_Game/Blueprint/Items/EItems` _iteminfo_eitem
              (:`NewEnumerator0`
                (`/Game/_Game/Blueprint/Core/GS_ShareYourTreat.Add score` (`self.GameStateRef`) 100.0 :!label _label_6)
                (`self.PlayVoiceline` "NewEnumerator2" :!label _label_7)
                (`SkeletalMeshComponent.PlayAnimation` (`self.Mesh`) (`|GetArrayItem` (`self.Montages`) (select `int` (`self.AnimIndex`) :`0` 1 :`1` 4 :`2` 7 :`3` 10 :`4` 13)) false)
                (`KismetSystemLibrary.Delay` 2.0)
                (`/Game/_Game/Blueprint/Environment/Door_BP.CloseDoor` (`self.DoorRef`))
                (`KismetSystemLibrary.Delay` 1.0)
                (`self.K2_DestroyActor`))
              (:`NewEnumerator7`
                (goto _label_6))
              (:`NewEnumerator8`
                (if (>= (select `int` (`self.AnimIndex`) :`0` -1 :`1` 5 :`2` 7 :`3` 4 :`4` 3) 0)
                  (`self.SetEyesValues`))
                (`self.FireParticles`)
                (`/Game/_Game/Blueprint/Core/GS_ShareYourTreat.Add score` (`self.GameStateRef`) 500.0)
                (goto _label_7))
              (:`NewEnumerator9`
                (goto _label_6))
              (:`NewEnumerator1`
                (`/Game/_Game/Blueprint/Core/GS_ShareYourTreat.Subtract Score` (`self.GameStateRef`) 500.0)
                (`self.PlayVoiceline` "NewEnumerator1")
                (`SkeletalMeshComponent.PlayAnimation` (`self.Mesh`) (`|GetArrayItem` (`self.Montages`) (select `int` (`self.AnimIndex`) :`0` 2 :`1` 5 :`2` 8 :`3` 11 :`4` 14)) false)
                (`KismetSystemLibrary.Delay` 5.5)
                (`/Game/_Game/Blueprint/Environment/Door_BP.CloseDoor` (`self.DoorRef`))
                (`KismetSystemLibrary.Delay` 1.0)
                (`self.K2_DestroyActor`))))
          (:`NewEnumerator4`
            (switch `/Game/_Game/Blueprint/Items/EItems` _iteminfo_eitem
              (:`NewEnumerator0`
                (`/Game/_Game/Blueprint/Core/GS_ShareYourTreat.Add score` (`self.GameStateRef`) 100.0 :!label _label_8)
                (`self.PlayVoiceline` "NewEnumerator2" :!label _label_9)
                (`SkeletalMeshComponent.PlayAnimation` (`self.Mesh`) (`|GetArrayItem` (`self.Montages`) (select `int` (`self.AnimIndex`) :`0` 1 :`1` 4 :`2` 7 :`3` 10 :`4` 13)) false)
                (`KismetSystemLibrary.Delay` 2.0)
                (`/Game/_Game/Blueprint/Environment/Door_BP.CloseDoor` (`self.DoorRef`))
                (`KismetSystemLibrary.Delay` 1.0)
                (`self.K2_DestroyActor`))
              (:`NewEnumerator7`
                (goto _label_8))
              (:`NewEnumerator8`
                (goto _label_8))
              (:`NewEnumerator9`
                (if (>= (select `int` (`self.AnimIndex`) :`0` -1 :`1` 5 :`2` 7 :`3` 4 :`4` 3) 0)
                  (`self.SetEyesValues`))
                (`self.FireParticles`)
                (`/Game/_Game/Blueprint/Core/GS_ShareYourTreat.Add score` (`self.GameStateRef`) 500.0)
                (goto _label_9))
              (:`NewEnumerator1`
                (`/Game/_Game/Blueprint/Core/GS_ShareYourTreat.Subtract Score` (`self.GameStateRef`) 500.0)
                (`self.PlayVoiceline` "NewEnumerator1")
                (`SkeletalMeshComponent.PlayAnimation` (`self.Mesh`) (`|GetArrayItem` (`self.Montages`) (select `int` (`self.AnimIndex`) :`0` 2 :`1` 5 :`2` 8 :`3` 11 :`4` 14)) false)
                (`KismetSystemLibrary.Delay` 5.5)
                (`/Game/_Game/Blueprint/Environment/Door_BP.CloseDoor` (`self.DoorRef`))
                (`KismetSystemLibrary.Delay` 1.0)
                (`self.K2_DestroyActor`))))))
      (:`else`))))

(fn `FireParticles`
  (bind _particlesref (`self.ParticlesRef`)
    (:`then`
      (`NiagaraComponent.SetPaused` _particlesref false))
    (:`else`)))

(fn `PlayVoiceline`
  (params (Voiceline :type "/Game/_Game/Blueprint/NPC/EVoiceLines Enum" :default "NewEnumerator0"))
  (bind (_hi _thanks _spray _time) (break `/Game/_Game/Blueprint/NPC/FVoices` (`BlueprintMapLibrary.Map_Find` (`self.Voices`) (`self.AnimIndex`))))
  (if (`.ReturnValue` (`BlueprintMapLibrary.Map_Find` (`self.Voices`) (`self.AnimIndex`)))
    (switch `/Game/_Game/Blueprint/NPC/EVoiceLines` Voiceline
      (:`NewEnumerator0`
        (bind _returnvalue (`GameplayStatics.SpawnSoundAttached` _hi (`self.Mesh`) "None" (0.0 0.0 0.0) (struct) "KeepRelativeOffset" false 1.0 1.0 0.0 null null))
        (set `AudioComponent.AttenuationSettings` "/Game/_Assets/Audio/Attenuation/SA_Voice.SA_Voice" _returnvalue)
        (`AudioComponent.Play` _returnvalue 0.0))
      (:`NewEnumerator1`
        (bind _returnvalue_2 (`GameplayStatics.SpawnSoundAttached` _thanks (`self.Mesh`) "None" (0.0 0.0 0.0) (struct) "KeepRelativeOffset" false 1.0 1.0 0.0 null null))
        (set `AudioComponent.AttenuationSettings` "/Game/_Assets/Audio/Attenuation/SA_Voice.SA_Voice" _returnvalue_2)
        (`AudioComponent.Play` _returnvalue_2 0.0))
      (:`NewEnumerator2`
        (bind _returnvalue_3 (`GameplayStatics.SpawnSoundAttached` _spray (`self.Mesh`) "None" (0.0 0.0 0.0) (struct) "KeepRelativeOffset" false 1.0 1.0 0.0 null null))
        (set `AudioComponent.AttenuationSettings` "/Game/_Assets/Audio/Attenuation/SA_Voice.SA_Voice" _returnvalue_3)
        (`AudioComponent.Play` _returnvalue_3 0.2))
      (:`NewEnumerator3`
        (bind _returnvalue_4 (`GameplayStatics.SpawnSoundAttached` _time (`self.Mesh`) "None" (0.0 0.0 0.0) (struct) "KeepRelativeOffset" false 1.0 1.0 0.0 null null))
        (set `AudioComponent.AttenuationSettings` "/Game/_Assets/Audio/Attenuation/SA_Voice.SA_Voice" _returnvalue_4)
        (`AudioComponent.Play` _returnvalue_4 0.0)))))

(fn `SetEyesValues`
  (`MaterialInstanceDynamic.SetVectorParameterValue` (`self.EyesMaterial`) "color" (`.EyesColor_29_47918EA342E9695AA1DD6E89D72D7758` (break `/Game/_Game/Blueprint/NPC/FCreatureStruct` (`self.CharInfo`))))
  (`MaterialInstanceDynamic.SetScalarParameterValue` (`self.EyesMaterial`) "scale" 50.0)
  (`PrimitiveComponent.SetMaterial` (`self.Mesh`) (select `int` (`self.AnimIndex`) :`0` -1 :`1` 5 :`2` 7 :`3` 4 :`4` 3) (`self.EyesMaterial`)))

(fn `SetLightValues`)

(fn `SpawnParticles`
  (bind ((`Particle_32_6AB37DE24BE09F208DC4A1B4B9C9974D` _particle)) (break `/Game/_Game/Blueprint/NPC/FCreatureStruct` (`self.CharInfo`)))
  (`/Engine/EditorBlueprintResources/StandardMacros.IsValid` _particle
    (:`Is Valid`
      (bind _returnvalue (`NiagaraFunctionLibrary.SpawnSystemAtLocation` _particle (`self.K2_GetActorLocation`) (struct) (1.0 1.0 1.0) true true "None" false))
      (bind _output_get (set `self.ParticlesRef` _returnvalue))
      (`NiagaraComponent.SetPaused` _output_get true)
      (`KismetSystemLibrary.PrintString` "SPAWNED"))))

(fn `UserConstructionScript`
  (locals (RandomInt :type Integer :default 0))
  (bind _output_get (set `self.RandomInt` (`KismetMathLibrary.RandomInteger` 5)))
  (switch `int` _output_get
    (:`0`
      (`SkeletalMeshComponent.SetSkeletalMeshAsset` (`self.Mesh`) "/Game/_Assets/Meshes/Boy2/Boy_2_2.Boy_2_2"))
    (:`1`
      (`SkeletalMeshComponent.SetSkeletalMeshAsset` (`self.Mesh`) "/Game/_Assets/Meshes/Boy3/Boy_3_6_Materials_Textures_Rigged_.Boy_3_6_Materials_Textures_Rigged_"))
    (:`2`
      (`SkeletalMeshComponent.SetSkeletalMeshAsset` (`self.Mesh`) "/Game/_Assets/Meshes/Boy4/Boy_4_Materials_Textures_Rigged_.Boy_4_Materials_Textures_Rigged_"))
    (:`3`
      (`SkeletalMeshComponent.SetSkeletalMeshAsset` (`self.Mesh`) "/Game/_Assets/Meshes/Girl1/Girl1_2.Girl1_2"))
    (:`4`
      (`SkeletalMeshComponent.SetSkeletalMeshAsset` (`self.Mesh`) "/Game/_Assets/Meshes/Girl2/Girl2_Materials_Textures_Rigged_.Girl2_Materials_Textures_Rigged_")))
  (set `self.AnimIndex` (`self.RandomInt`)))
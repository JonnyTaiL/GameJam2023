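; NPC spawner actor that creates one human or other NPC after a randomized delay from BeginPlay, and again whenever StartCount is called.
; A one-shot timer triggers a weighted HumanChance roll, choosing either the "human" row or a random IDName row from DT_Npc.
; The row's EnemyType spawns slightly above the spawner, receiving the row data, DoorRef and a spawner reference.
; An unconnected reroll loop that excludes "human" never runs.
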(event `StartCount`
  (bind _timedelay (`self.TimeDelay`))
  (bind _returnvalue (`KismetSystemLibrary.K2_SetTimerDelegate` (delegate `spawn creature`) (`KismetMathLibrary.RandomFloatInRange` _timedelay (+ _timedelay 4.0)) :!label _label))
  (set `self.TimerHandle` _returnvalue))

(event `self.ReceiveBeginPlay`
  (goto _label))

(event `spawn creature`
  (`self.SpawnCreature` (`self.HumanChance`)))

(event `SpawnCreature`
  (params (HumanChance :type "Float (double-precision)"))
  (if (`KismetMathLibrary.RandomBoolWithWeight` HumanChance)
    (bind _returnvalue (`|GetDataTableRow` "/Game/_Game/Blueprint/NPC/DT_Npc.DT_Npc" "human")
      (:`then`
        (`|SpawnActorFromClass` (`.EnemyType_9_4715B60D47F5B8C7CD2FB0827D4E195E` (break `/Game/_Game/Blueprint/NPC/FCreatureStruct` _returnvalue)) (`KismetMathLibrary.MakeTransform` (+ (`self.K2_GetActorLocation`) (0.0 0.0 95.0)) (`self.K2_GetActorRotation`)) "Undefined" "OverrideRootScale" null _returnvalue self (`self.DoorRef`) null)))
    (else
      (bind _returnvalue_2 (`|GetDataTableRow` "/Game/_Game/Blueprint/NPC/DT_Npc.DT_Npc" (`KismetArrayLibrary.Array_Random` (`self.IDName`)))
        (:`then`
          (`|SpawnActorFromClass` (`.EnemyType_9_4715B60D47F5B8C7CD2FB0827D4E195E` (break `/Game/_Game/Blueprint/NPC/FCreatureStruct` _returnvalue_2)) (`KismetMathLibrary.MakeTransform` (+ (`self.K2_GetActorLocation`) (0.0 0.0 95.0)) (`self.K2_GetActorRotation`)) "Undefined" "OverrideRootScale" null _returnvalue_2 self (`self.DoorRef`) null))))))

(fn `UserConstructionScript`)
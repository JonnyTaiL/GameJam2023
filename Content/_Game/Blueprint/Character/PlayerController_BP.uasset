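; Player controller that creates the main HUD, caches the player character and game state, and handles first-person input through Enhanced Input.
; Each tick, LookAt traces from the camera and sends look-at and stop-look-at messages as the targeted actor changes.
; Interact messages the targeted ItemMaster_BP when CurrentItem passes its check, while Use and Cancel message the current item.
; Tick also prints the targeted actor and score for debugging.
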(event `self.ReceiveBeginPlay`
  (bind _returnvalue (subsystem `EnhancedInputLocalPlayerSubsystem`))
  (`|ExecutionSequence`
    (:`then_0`
      (bind _asplayer_character_bp (cast `/Game/_Game/Blueprint/Character/PlayerCharacter_BP` (`GameplayStatics.GetPlayerCharacter` 0)))
      (set `self.PlayerRef` _asplayer_character_bp)
      (bind _returnvalue_2 (`|CreateWidget` "/Game/_Game/Blueprint/UI/UI_Main.UI_Main_C" self))
      (bind _output_get (set `self.MainWidgetRef` _returnvalue_2))
      (`UserWidget.AddToViewport` _output_get 0)
      (set `/Game/_Game/Blueprint/Character/PlayerCharacter_BP.ControllerRef` self (`self.PlayerRef`))
      (bind _asgs_share_your_treat (cast `/Game/_Game/Blueprint/Core/GS_ShareYourTreat` (`GameplayStatics.GetGameState`)))
      (set `self.GameStateRef` _asgs_share_your_treat))
    (:`then_1`
      (`/Engine/EditorBlueprintResources/StandardMacros.IsValid` _returnvalue
        (:`Is Valid`
          (`EnhancedInputSubsystemInterface.AddMappingContext` _returnvalue "/Game/_Game/Blueprint/Character/Inputs/IMC_PlayerInputs.IMC_PlayerInputs" 0 (struct)))))))

(event `EnhancedInput|/Game/_Game/Blueprint/Character/Inputs/IA_Look`
  (params (ActionValue :type "Vector2D Structure") (ElapsedSeconds :type "Float (double-precision)") (TriggeredSeconds :type "Float (double-precision)") (InputAction :type "InputAction Object Reference" :default "/Game/_Game/Blueprint/Character/Inputs/IA_Look.IA_Look"))
  (bind _playerref (`self.PlayerRef`))
  ;[1 1 1] Look around
  (:`Triggered`
    (`Pawn.AddControllerYawInput` _playerref ActionValue_X)
    (`Pawn.AddControllerPitchInput` _playerref (* ActionValue_Y -1.0))))

(event `EnhancedInput|/Game/_Game/Blueprint/Character/Inputs/IA_Move`
  (params (ActionValue :type "Vector2D Structure") (ElapsedSeconds :type "Float (double-precision)") (TriggeredSeconds :type "Float (double-precision)") (InputAction :type "InputAction Object Reference" :default "/Game/_Game/Blueprint/Character/Inputs/IA_Move.IA_Move"))
  (bind (_returnvalue_roll _returnvalue_pitch _returnvalue_yaw) (`KismetMathLibrary.BreakRotator` (`self.GetControlRotation`)))
  (bind (_returnvalue_roll_2 _returnvalue_pitch_2 _returnvalue_yaw_2) (`KismetMathLibrary.BreakRotator` (`self.GetControlRotation`)))
  ;[1 1 1] Movement
  (:`Triggered`
    (`Pawn.AddMovementInput` (`self.PlayerRef`) (`KismetMathLibrary.GetRightVector` (`KismetMathLibrary.MakeRotator` _returnvalue_roll 0.0 _returnvalue_yaw)) ActionValue_X false)
    (`Pawn.AddMovementInput` (`self.PlayerRef`) (`KismetMathLibrary.GetForwardVector` (`KismetMathLibrary.MakeRotator` 0.0 0.0 _returnvalue_yaw_2)) ActionValue_Y false)))

(event `EnhancedInput|/Game/_Game/Blueprint/Character/Inputs/IA_Interact`
  (params (ActionValue :type Boolean) (ElapsedSeconds :type "Float (double-precision)") (TriggeredSeconds :type "Float (double-precision)") (InputAction :type "InputAction Object Reference" :default "/Game/_Game/Blueprint/Character/Inputs/IA_Interact.IA_Interact"))
  (:`Started`
    (if (== (`self.CurrentItem`) null)
      (bind _lookatactor (`self.LookAtActor`)
        (:`then`
          (bind _asitem_master_bp (cast `/Game/_Game/Blueprint/Items/ItemMaster_BP` _lookatactor))
          (message `/Game/_Game/Blueprint/Core/I_Interact.StopLookAt` _asitem_master_bp self)
          (message `/Game/_Game/Blueprint/Core/I_Interact.InteractWith` _asitem_master_bp self))
        (:`else`)))))

(event `EnhancedInput|/Game/_Game/Blueprint/Character/Inputs/IA_Cancel`
  (params (ActionValue :type Boolean) (ElapsedSeconds :type "Float (double-precision)") (TriggeredSeconds :type "Float (double-precision)") (InputAction :type "InputAction Object Reference" :default "/Game/_Game/Blueprint/Character/Inputs/IA_Cancel.IA_Cancel"))
  (:`Started`
    (bind _currentitem (`self.CurrentItem`)
      (:`then`
        (message `/Game/_Game/Blueprint/Core/I_Interact.Cancel` _currentitem self))
      (:`else`))))

(event `self.ReceiveTick`
  (params (DeltaSeconds :type "Float (single-precision)"))
  (set `self.Delta Seconds` DeltaSeconds)
  (`|ExecutionSequence`
    (:`then_0`
      (`self.LookAt`))
    (:`then_1`
      ;[1 1 1] DEBUG
      (`KismetSystemLibrary.PrintString` (`KismetStringLibrary.Concat_StrStr` "LookAtActor - " (`KismetSystemLibrary.GetDisplayName` (`self.LookAtActor`))) true true (struct :`G` 0.66 :`B` 1.0 :`A` 1.0) (`self.Delta Seconds`))
      (`KismetSystemLibrary.PrintString` (`KismetStringLibrary.Concat_StrStr` "Score - " (`KismetStringLibrary.Conv_DoubleToString` (`/Game/_Game/Blueprint/Core/GS_ShareYourTreat.Score` (`self.GameStateRef`)))) true true (struct :`R` 1.0 :`B` 0.019001 :`A` 1.0) (`self.Delta Seconds`)))))

(event `EnhancedInput|/Game/_Game/Blueprint/Character/Inputs/IA_Use`
  (params (ActionValue :type Boolean) (ElapsedSeconds :type "Float (double-precision)") (TriggeredSeconds :type "Float (double-precision)") (InputAction :type "InputAction Object Reference" :default "/Game/_Game/Blueprint/Character/Inputs/IA_Use.IA_Use"))
  (:`Started`
    (bind _currentitem (`self.CurrentItem`)
      (:`then`
        (message `/Game/_Game/Blueprint/Core/I_Interact.Use` _currentitem self))
      (:`else`))))

(fn `LookAt`
  (locals (Local_LookAtActor :type "Actor Object Reference"))
  (bind _camera (`/Game/_Game/Blueprint/Character/PlayerCharacter_BP.Camera` (`self.PlayerRef`)))
  (bind _returnvalue (`SceneComponent.K2_GetComponentLocation` _camera))
  (bind (_outhit _returnvalue_2) (`KismetSystemLibrary.LineTraceSingle` _returnvalue (+ _returnvalue (* (`SceneComponent.GetForwardVector` _camera) (`self.InteractLength`))) "TraceTypeQuery1" true))
  (if _returnvalue_2
    (bind (_bblockinghit _binitialoverlap _time _distance _location _impactpoint _normal _impactnormal _physmat _hitactor) (`GameplayStatics.BreakHitResult` _outhit))
    (if (!= (`self.LookAtActor`) _hitactor)
      (bind _output_get (set `local.Local_LookAtActor` _hitactor))
      (if (!= _output_get (`self.LookAtActor`))
        (message `/Game/_Game/Blueprint/Core/I_Interact.StopLookAt` (`self.LookAtActor`) self))
      (set `self.LookAtActor` _hitactor)
      (message `/Game/_Game/Blueprint/Core/I_Interact.LookAt` (`self.LookAtActor`) self))
    (else
      (bind _lookatactor (`self.LookAtActor`)
        (:`then`
          (message `/Game/_Game/Blueprint/Core/I_Interact.StopLookAt` _lookatactor self))
        (:`else`
          _))
      (set `self.LookAtActor` null))))

(fn `RayCast`
  (bind _camera (`/Game/_Game/Blueprint/Character/PlayerCharacter_BP.Camera` (`self.PlayerRef`)))
  (bind _returnvalue (`SceneComponent.K2_GetComponentLocation` _camera))
  (bind _outhit (`KismetSystemLibrary.LineTraceSingle` _returnvalue (+ _returnvalue (* (`SceneComponent.GetForwardVector` _camera) (`self.InteractLength`))) "TraceTypeQuery1" true)))

(fn `UserConstructionScript`)
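; Player character Blueprint that tracks distance walked to time footstep surface checks.
; Each Tick subtracts speed times delta time from a step-distance counter, which resets to the step length when it runs out.
; At each step, a short downward Visibility trace with debug drawing reads the physical material's surface type.
; The switch on that surface type has no responses wired, so no footstep effect plays yet.
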(event `self.ReceiveTick`
  (params (DeltaSeconds :type "Float (single-precision)"))
  (set `self.Delta Seconds` DeltaSeconds)
  (set `self.Speed` (`KismetMathLibrary.VSize` (`self.GetVelocity`)))
  (`self.CalculateStepDist`)
  (if (<= (`self.StepTemp`) 0.0)
    (`self.StepCast`)
    (set `self.StepTemp` (`self.StepLength`))))

(fn `CalculateStepDist`
  (set `self.StepTemp` (- (`self.StepTemp`) (* (`self.Speed`) (`self.Delta Seconds`)))))

(fn `StepCast`
  (bind _returnvalue (`self.K2_GetActorLocation`))
  (bind (_outhit _returnvalue_2) (`KismetSystemLibrary.LineTraceSingle` :`Start` (- _returnvalue (0.0 0.0 60.0)) :`End` (- _returnvalue (0.0 0.0 100.0)) :`TraceChannel` "TraceTypeQuery1" :`DrawDebugType` "ForDuration"))
  (if _returnvalue_2
    (switch `EPhysicalSurface` (`PhysicalMaterial.SurfaceType` (`.PhysMat` (`GameplayStatics.BreakHitResult` _outhit))))))

(fn `UserConstructionScript`)
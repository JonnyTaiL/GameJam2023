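; AntiWitch is a usable item that sprays the NPC the player is looking at.
; On Use, it casts the controller's look-at actor to NPC_Master and calls InteractWith only if that NPC has not been interacted with.
; It then spawns a spray particle effect and an attached sound at its Scene component, holding Using true for a short delay before destroying the emitter.
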(event `/Game/_Game/Blueprint/Core/I_Interact.Use`
  (params (ControllerRef :type "/Game/_Game/Blueprint/Character/PlayerController_BP Object Reference"))
  (bind _asnpc_master (cast `/Game/_Game/Blueprint/NPC/NPC_Master` (`/Game/_Game/Blueprint/Character/PlayerController_BP.LookAtActor` ControllerRef)))
  (if (not (`/Game/_Game/Blueprint/NPC/NPC_Master.Interacted` _asnpc_master))
    (`/Game/_Game/Blueprint/Core/I_Interact.InteractWith` _asnpc_master ControllerRef)
    (set `self.Using` true)
    (bind _returnvalue (`NiagaraFunctionLibrary.SpawnSystemAtLocation` "/Game/_Game/Blueprint/VFX/NE_Spray_System.NE_Spray_System" (`SceneComponent.K2_GetComponentLocation` (`self.Scene`)) (struct :`Pitch` 90.0)))
    (set `self.Emitter` _returnvalue)
    (bind _returnvalue_2 (`GameplayStatics.SpawnSoundAttached` "/Game/_Assets/Audio/Metasounds/MS_Spray.MS_Spray" (`self.Scene`) "None" (0.0 0.0 0.0) (struct) "KeepRelativeOffset" false 1.0 1.0 0.0 null null))
    (`AudioComponent.Play` _returnvalue_2 0.0)
    (`KismetSystemLibrary.Delay` 0.5)
    (`ActorComponent.K2_DestroyComponent` (`self.Emitter`))
    (set `self.Using` false)))

(fn `UserConstructionScript`
  (`parent.UserConstructionScript`))
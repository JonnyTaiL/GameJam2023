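; HolyWater_BP is a holy water item that, when used, interacts with the NPC the player is looking at.
; Its Use event takes a controller reference, casts that controller's LookAtActor to NPC_Master and calls InteractWith on it, passing the controller along.
; Nothing happens if the target is not an NPC_Master, and any effect specific to holy water lives outside this graph.
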(event `/Game/_Game/Blueprint/Core/I_Interact.Use`
  (params (ControllerRef :type "/Game/_Game/Blueprint/Character/PlayerController_BP Object Reference"))
  (bind _asnpc_master (cast `/Game/_Game/Blueprint/NPC/NPC_Master` (`/Game/_Game/Blueprint/Character/PlayerController_BP.LookAtActor` ControllerRef)))
  (`/Game/_Game/Blueprint/Core/I_Interact.InteractWith` _asnpc_master ControllerRef))

(fn `UserConstructionScript`
  (`parent.UserConstructionScript`))
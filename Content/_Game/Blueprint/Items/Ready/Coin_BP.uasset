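; Coin item that spins on use and lands on heads or tails, with nearby NPC types able to rig the result.
; While not moving, React looks up the NPC in DT_Npc to keep the flip random or force a side by type, and StopReact restores randomness.
; Use rolls the side when random, then the Spin timeline rotates the mesh and snaps its yaw to the result.
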(event `/Game/_Game/Blueprint/Core/I_Reaction.React`
  (params (IdName :type Name))
  (`parent.React` IdName)
  (if (not (`self.Moving`))
    (bind _returnvalue (`|GetDataTableRow` "/Game/_Game/Blueprint/NPC/DT_Npc.DT_Npc" IdName)
      (:`then`
        (switch `/Game/_Game/Blueprint/NPC/E_NPCTypes` (`.Types_24_DFB46F504CB588E60C2E12848E012112` (break `/Game/_Game/Blueprint/NPC/FCreatureStruct` _returnvalue))
          (:`NewEnumerator0`
            (set `self.Random?` true))
          (:`NewEnumerator1`
            (set `self.Random?` true))
          (:`NewEnumerator2`
            (set `self.Random?` false)
            (set `self.Tail?` true))
          (:`NewEnumerator3`
            (set `self.Random?` false)
            (set `self.Tail?` true))
          (:`NewEnumerator4`
            (set `self.Random?` false)
            (set `self.Tail?` false)))
        (`KismetSystemLibrary.PrintString` (`KismetStringLibrary.Conv_BoolToString` (`self.Tail?`)))))))

(event `/Game/_Game/Blueprint/Core/I_Reaction.StopReact`
  (params (IdName :type Name))
  (`parent.StopReact` IdName)
  (if (not (`self.Moving`))
    (bind _returnvalue (`|GetDataTableRow` "/Game/_Game/Blueprint/NPC/DT_Npc.DT_Npc" IdName)
      (:`then`
        (switch `/Game/_Game/Blueprint/NPC/E_NPCTypes` (`.Types_24_DFB46F504CB588E60C2E12848E012112` (break `/Game/_Game/Blueprint/NPC/FCreatureStruct` _returnvalue))
          (:`NewEnumerator0`
            _)
          (:`NewEnumerator1`
            _)
          (:`NewEnumerator2`
            _)
          (:`NewEnumerator3`
            _)
          (:`NewEnumerator4`
            _))
        (set `self.Random?` true)))))

(event `/Game/_Game/Blueprint/Core/I_Interact.Use`
  (params (ControllerRef :type "/Game/_Game/Blueprint/Character/PlayerController_BP Object Reference"))
  (bind _staticmesh (`self.StaticMesh`))
  (bind (_relativerotation_roll _relativerotation_pitch) (`KismetMathLibrary.BreakRotator` (`SceneComponent.RelativeRotation` (`self.StaticMesh`))))
  (bind (_relativerotation_roll_2 _relativerotation_pitch_2) (`KismetMathLibrary.BreakRotator` (`SceneComponent.RelativeRotation` _staticmesh)))
  (if (`self.Random?`)
    (set `self.Tail?` (`KismetMathLibrary.RandomBoolWithWeight` 0.5))
    (bind (_direction _spin) (`Timeline|Spin` :!via `PlayFromStart` :!label _label)
      (:`Update`
        (`SceneComponent.K2_AddRelativeRotation` (`self.StaticMesh`) (`KismetMathLibrary.MakeRotator` 0.0 0.0 (* _spin 50.0)) false false))
      (:`Finished`
        (if (`self.Tail?`)
          (`SceneComponent.K2_SetRelativeRotation` _staticmesh (`KismetMathLibrary.MakeRotator` _relativerotation_roll_2 _relativerotation_pitch_2) false false)
          (else
            (`SceneComponent.K2_SetRelativeRotation` (`self.StaticMesh`) (`KismetMathLibrary.MakeRotator` _relativerotation_roll _relativerotation_pitch 180.0) false false)))))
    (else
      (goto _label :!via `PlayFromStart`))))

(fn `UserConstructionScript`
  (`parent.UserConstructionScript`))
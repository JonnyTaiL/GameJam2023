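; DreamCatcher item that glows when it reacts to a supernatural NPC, acting as a detector while it is not moving.
; React looks up the NPC in DT_Npc and calls AddLight for Demon, Witch, Ghost or Werewolf types.
; A timeline drives point light intensity and sets the Enabled flag by its finishing direction.
; StopReact reverses that timeline to fade the light for any NPC found in the table.
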(event `AddLight`
  (if (not (`self.Enabled?`))
    (bind (_direction _intensity) (`Timeline|Int` :!label _label)
      (:`Update`
        (`LightComponent.SetIntensity` (`self.PointLight`) _intensity))
      (:`Finished`
        (switch `ETimelineDirection` _direction
          (:`Forward`
            (set `self.Enabled?` true))
          (:`Backward`
            (set `self.Enabled?` false)))))))

(event `RemoveLight`
  (goto _label :!via `Reverse`))

(event `/Game/_Game/Blueprint/Core/I_Reaction.React`
  (params (IdName :type Name))
  (`parent.React` IdName)
  (if (not (`self.Moving`))
    (bind _returnvalue (`|GetDataTableRow` "/Game/_Game/Blueprint/NPC/DT_Npc.DT_Npc" IdName)
      (:`then`
        (switch `/Game/_Game/Blueprint/NPC/E_NPCTypes` (`.Types_24_DFB46F504CB588E60C2E12848E012112` (break `/Game/_Game/Blueprint/NPC/FCreatureStruct` _returnvalue))
          (:`NewEnumerator1`
            _)
          (:`NewEnumerator2`
            _)
          (:`NewEnumerator3`
            _)
          (:`NewEnumerator4`
            _))
        (`self.AddLight`)))))

(event `/Game/_Game/Blueprint/Core/I_Reaction.StopReact`
  (params (IdName :type Name))
  (`parent.StopReact` IdName)
  (bind _returnvalue (`|GetDataTableRow` "/Game/_Game/Blueprint/NPC/DT_Npc.DT_Npc" IdName)
    (:`then`
      (switch `/Game/_Game/Blueprint/NPC/E_NPCTypes` (`.Types_24_DFB46F504CB588E60C2E12848E012112` (break `/Game/_Game/Blueprint/NPC/FCreatureStruct` _returnvalue))
        (:`NewEnumerator0`
          _)
        (:`NewEnumerator1`
          _)
        (:`NewEnumerator2`
          _)
        (:`NewEnumerator3`
          _)
        (:`NewEnumerator4`
          _))
      (`self.RemoveLight`))))

(fn `UserConstructionScript`
  (`parent.UserConstructionScript`))
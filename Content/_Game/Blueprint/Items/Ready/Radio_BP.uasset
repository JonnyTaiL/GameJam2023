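; Radio item Blueprint that starts playing audio in reaction to supernatural Demon or Ghost NPCs while it is not moving.
; React looks up the NPC's type in DT_Npc by IdName and calls Start to fade the audio in.
; StopReact calls End to fade it out when the NPC's row is found.
; BeginPlay silences the audio immediately, and both react events also run their parent implementations.
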(event `Start`
  (`AudioComponent.FadeIn` (`self.Audio`) 2.0 1.0 0.0 "Linear"))

(event `self.ReceiveBeginPlay`
  (`AudioComponent.FadeOut` (`self.Audio`) 0.0 0.0 "Linear"))

(event `End`
  (`AudioComponent.FadeOut` (`self.Audio`) 2.0 0.0 "Linear"))

(event `/Game/_Game/Blueprint/Core/I_Reaction.React`
  (params (IdName :type Name))
  (`parent.React` IdName)
  (if (not (`self.Moving`))
    (bind _returnvalue (`|GetDataTableRow` "/Game/_Game/Blueprint/NPC/DT_Npc.DT_Npc" IdName)
      (:`then`
        (switch `/Game/_Game/Blueprint/NPC/E_NPCTypes` (`.Types_24_DFB46F504CB588E60C2E12848E012112` (break `/Game/_Game/Blueprint/NPC/FCreatureStruct` _returnvalue))
          (:`NewEnumerator1`
            _)
          (:`NewEnumerator3`
            _))
        (`self.Start`)))))

(event `/Game/_Game/Blueprint/Core/I_Reaction.StopReact`
  (params (IdName :type Name))
  (`parent.StopReact` IdName)
  (bind _returnvalue (`|GetDataTableRow` "/Game/_Game/Blueprint/NPC/DT_Npc.DT_Npc" IdName)
    (:`then`
      (switch `/Game/_Game/Blueprint/NPC/E_NPCTypes` (`.Types_24_DFB46F504CB588E60C2E12848E012112` (break `/Game/_Game/Blueprint/NPC/FCreatureStruct` _returnvalue))
        (:`NewEnumerator0`
          _)
        (:`NewEnumerator1`
          _)
        (:`NewEnumerator2`
          _)
        (:`NewEnumerator3`
          _)
        (:`NewEnumerator4`
          _))
      (`self.End`))))

(fn `UserConstructionScript`
  (`parent.UserConstructionScript`))
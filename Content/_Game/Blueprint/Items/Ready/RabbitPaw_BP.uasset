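; RabbitPaw is an item Blueprint for a rabbit paw that swings when it reacts to a supernatural NPC.
; React looks up the NPC type in DT_Npc and, unless the item is moving, starts the Swing timeline for Demon, Witch, Ghost or Werewolf.
; Swing drives the static mesh's pitch.
; StopReact calls End, which stops the swing and plays a Return timeline that lerps pitch back to zero.
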(event `Start`
  (bind _staticmesh (`self.StaticMesh`))
  (bind (_relativerotation_roll _relativerotation_pitch _relativerotation_yaw) (`KismetMathLibrary.BreakRotator` (`SceneComponent.RelativeRotation` _staticmesh)))
  (bind (_direction _swing) (`Timeline|Swing` :!via `PlayFromStart` :!label _label)
    (:`Update`
      (`SceneComponent.K2_SetRelativeRotation` _staticmesh (`KismetMathLibrary.MakeRotator` _relativerotation_roll _swing _relativerotation_yaw) false false))))

(event `End`
  (bind (_relativerotation_roll _relativerotation_pitch _relativerotation_yaw) (`KismetMathLibrary.BreakRotator` (`SceneComponent.RelativeRotation` (`self.StaticMesh`))))
  (`|ExecutionSequence`
    (:`then_0`
      (goto _label :!via `Stop`))
    (:`then_1`
      (bind (_direction _prog) (`Timeline|Return` :!via `PlayFromStart`)
        (:`Update`
          (`SceneComponent.K2_SetRelativeRotation` (`self.StaticMesh`) (`KismetMathLibrary.MakeRotator` _relativerotation_roll (`KismetMathLibrary.Lerp` _relativerotation_pitch 0.0 _prog) _relativerotation_yaw) false false))))))

(event `/Game/_Game/Blueprint/Core/I_Reaction.React`
  (params (IdName :type Name))
  (`parent.React` IdName)
  (if (not (`self.Moving`))
    (bind _returnvalue (`|GetDataTableRow` "/Game/_Game/Blueprint/NPC/DT_Npc.DT_Npc" IdName)
      (:`then`
        (switch `/Game/_Game/Blueprint/NPC/E_NPCTypes` (`.Types_24_DFB46F504CB588E60C2E12848E012112` (break `/Game/_Game/Blueprint/NPC/FCreatureStruct` _returnvalue))
          (:`NewEnumerator1`
            _)
          (:`NewEnumerator2`
            _)
          (:`NewEnumerator3`
            _)
          (:`NewEnumerator4`
            _))
        (`self.Start`)))))

(event `/Game/_Game/Blueprint/Core/I_Reaction.StopReact`
  (params (IdName :type Name))
  (`parent.StopReact` IdName)
  (bind _returnvalue (`|GetDataTableRow` "/Game/_Game/Blueprint/NPC/DT_Npc.DT_Npc" IdName)
    (:`then`
      (switch `/Game/_Game/Blueprint/NPC/E_NPCTypes` (`.Types_24_DFB46F504CB588E60C2E12848E012112` (break `/Game/_Game/Blueprint/NPC/FCreatureStruct` _returnvalue))
        (:`NewEnumerator0`
          _)
        (:`NewEnumerator1`
          _)
        (:`NewEnumerator2`
          _)
        (:`NewEnumerator3`
          _)
        (:`NewEnumerator4`
          _))
      (`self.End`))))

(fn `UserConstructionScript`
  (`parent.UserConstructionScript`))
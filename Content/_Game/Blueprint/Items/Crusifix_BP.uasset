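; Crucifix item Blueprint with React and StopReact events that respond to an NPC identified by row name.
; Each event looks up that NPC in the DT_Npc data table and switches on its type: Human, Demon, Witch, Ghost or Werewolf.
; Both events currently only print the matched type name, with no distinct behavior for starting or stopping the reaction.
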(event `/Game/_Game/Blueprint/Core/I_Reaction.React`
  (params (IdName :type Name))
  (bind _returnvalue (`|GetDataTableRow` "/Game/_Game/Blueprint/NPC/DT_Npc.DT_Npc" IdName)
    (:`then`
      (switch `/Game/_Game/Blueprint/NPC/E_NPCTypes` (`.Types_24_DFB46F504CB588E60C2E12848E012112` (break `/Game/_Game/Blueprint/NPC/FCreatureStruct` _returnvalue))
        (:`NewEnumerator0`
          (`KismetSystemLibrary.PrintString` "HUMAN" true true (struct :`G` 0.078467 :`B` 1.0 :`A` 1.0)))
        (:`NewEnumerator1`
          (`KismetSystemLibrary.PrintString` "DEMON" true true (struct :`G` 0.078467 :`B` 1.0 :`A` 1.0)))
        (:`NewEnumerator2`
          (`KismetSystemLibrary.PrintString` "WITCH" true true (struct :`G` 0.078467 :`B` 1.0 :`A` 1.0)))
        (:`NewEnumerator3`
          (`KismetSystemLibrary.PrintString` "GHOST" true true (struct :`G` 0.078467 :`B` 1.0 :`A` 1.0)))
        (:`NewEnumerator4`
          (`KismetSystemLibrary.PrintString` "WEREWOLF" true true (struct :`G` 0.078467 :`B` 1.0 :`A` 1.0)))))))

(event `/Game/_Game/Blueprint/Core/I_Reaction.StopReact`
  (params (IdName :type Name))
  (bind _returnvalue (`|GetDataTableRow` "/Game/_Game/Blueprint/NPC/DT_Npc.DT_Npc" IdName)
    (:`then`
      (switch `/Game/_Game/Blueprint/NPC/E_NPCTypes` (`.Types_24_DFB46F504CB588E60C2E12848E012112` (break `/Game/_Game/Blueprint/NPC/FCreatureStruct` _returnvalue))
        (:`NewEnumerator0`
          (`KismetSystemLibrary.PrintString` "HUMAN" true true (struct :`G` 0.078467 :`B` 1.0 :`A` 1.0)))
        (:`NewEnumerator1`
          (`KismetSystemLibrary.PrintString` "DEMON" true true (struct :`G` 0.078467 :`B` 1.0 :`A` 1.0)))
        (:`NewEnumerator2`
          (`KismetSystemLibrary.PrintString` "WITCH" true true (struct :`G` 0.078467 :`B` 1.0 :`A` 1.0)))
        (:`NewEnumerator3`
          (`KismetSystemLibrary.PrintString` "GHOST" true true (struct :`G` 0.078467 :`B` 1.0 :`A` 1.0)))
        (:`NewEnumerator4`
          (`KismetSystemLibrary.PrintString` "WEREWOLF" true true (struct :`G` 0.078467 :`B` 1.0 :`A` 1.0)))))))

(fn `UserConstructionScript`
  (`parent.UserConstructionScript`))
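; Base item Actor that the player can highlight, pick up into a grip and return to its spawner.
; Look-at events toggle custom depth on the mesh, while React events only print debug text.
; Interact and Cancel set or clear the controller's CurrentItem, guarded by a Moving flag.
; Timelines lerp the item from its continually updated transform to the player's ItemGrip or back to the Spawner, then snap-attach it.
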(event `/Game/_Game/Blueprint/Core/I_Interact.LookAt`
  (params (PlayerController :type "/Game/_Game/Blueprint/Character/PlayerController_BP Object Reference"))
  (`PrimitiveComponent.SetRenderCustomDepth` (`self.StaticMesh`) true))

(event `/Game/_Game/Blueprint/Core/I_Interact.StopLookAt`
  (params (PlayerController :type "/Game/_Game/Blueprint/Character/PlayerController_BP Object Reference"))
  (`PrimitiveComponent.SetRenderCustomDepth` (`self.StaticMesh`) false))

(event `/Game/_Game/Blueprint/Core/I_Interact.InteractWith`
  (params (PlayerController :type "/Game/_Game/Blueprint/Character/PlayerController_BP Object Reference"))
  (bind _itemgrip (`/Game/_Game/Blueprint/Character/PlayerCharacter_BP.ItemGrip` (`/Game/_Game/Blueprint/Character/PlayerController_BP.PlayerRef` PlayerController)))
  (if (not (`self.Moving`))
    (bind _output_get (set `self.Player Controller` PlayerController))
    (set `/Game/_Game/Blueprint/Character/PlayerController_BP.CurrentItem` self _output_get)
    (set `self.Moving` true)
    (bind (_direction _percent) (`Timeline|Slide` :!via `PlayFromStart`)
      (:`Update`
        (`self.K2_SetActorLocationAndRotation` (`KismetMathLibrary.VLerp` (`self.K2_GetActorLocation`) (`SceneComponent.K2_GetComponentLocation` _itemgrip) _percent) (`KismetMathLibrary.RLerp` (`self.K2_GetActorRotation`) (`SceneComponent.K2_GetComponentRotation` _itemgrip) _percent true)))
      (:`Finished`
        (`self.K2_AttachToComponent` (`/Game/_Game/Blueprint/Character/PlayerCharacter_BP.ItemGrip` (`/Game/_Game/Blueprint/Character/PlayerController_BP.PlayerRef` (`self.Player Controller`))) "None" "SnapToTarget" "SnapToTarget" "KeepRelative")
        (set `self.Moving` false)))))

(event `/Game/_Game/Blueprint/Core/I_Reaction.React`
  (params (IdName :type Name))
  (`KismetSystemLibrary.PrintString` "React" true true (struct :`R` 1.0 :`B` 0.105954 :`A` 1.0)))

(event `/Game/_Game/Blueprint/Core/I_Reaction.StopReact`
  (params (IdName :type Name))
  (`KismetSystemLibrary.PrintString` "Stop React" true true (struct :`R` 0.048198 :`G` 1.0 :`A` 1.0)))

(event `/Game/_Game/Blueprint/Core/I_Interact.Cancel`
  (params (ControllerRef :type "/Game/_Game/Blueprint/Character/PlayerController_BP Object Reference"))
  (bind _spawner (`self.Spawner`))
  (if (not (`self.Moving`))
    (bind _output_get (set `self.Player Controller` ControllerRef))
    (set `/Game/_Game/Blueprint/Character/PlayerController_BP.CurrentItem` null _output_get)
    (set `self.Moving` true)
    (bind (_direction _percent) (`Timeline|BackSlide` :!via `PlayFromStart`)
      (:`Update`
        (`self.K2_SetActorLocationAndRotation` (`KismetMathLibrary.VLerp` (`self.K2_GetActorLocation`) (`self.K2_GetActorLocation` _spawner) _percent) (`KismetMathLibrary.RLerp` (`self.K2_GetActorRotation`) (`self.K2_GetActorRotation` _spawner) _percent true)))
      (:`Finished`
        (`self.K2_AttachToActor` (`self.Spawner`) "None" "SnapToTarget" "SnapToTarget" "KeepRelative")
        (set `self.Moving` false)))))

(fn `UserConstructionScript`)
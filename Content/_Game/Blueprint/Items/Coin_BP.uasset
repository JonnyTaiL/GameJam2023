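; Coin item Blueprint that overrides its parent's React and StopReact events, with only placeholder debug responses so far.
; Both events call the parent, then, if the coin is not moving, look up the given IdName in the DT_Npc data table.
; The row's NPC type (Human, Demon, Witch, Ghost or Werewolf) selects which type name is printed, with identical logic in both events.
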(event `/Game/_Game/Blueprint/Core/I_Reaction.React`
  (params (IdName :type Name))
  (`parent.React` IdName)
  (if (not (`self.Moving`))
    (bind _returnvalue (`|GetDataTableRow` "/Game/_Game/Blueprint/NPC/DT_Npc.DT_Npc" IdName)
      (:`then`
        (switch `/Game/_Game/Blueprint/NPC/E_NPCTypes` (`.Types_24_DFB46F504CB588E60C2E12848E012112` (break `/Game/_Game/Blueprint/NPC/FCreatureStruct` _returnvalue))
          (:`NewEnumerator0`
            (`KismetSystemLibrary.PrintString` "HUMAN" true true (struct :`G` 0.078467 :`B` 1.0 :`A` 1.0)))
          (:`NewEnumerator1`
            (`KismetSystemLibrary.PrintString` "DEMON" true true (struct :`G` 0.078467 :`B` 1.0 :`A` 1.0)))
          (:`NewEnumerator2`
            (`KismetSystemLibrary.PrintString` "WITCH" true true (struct :`G` 0.078467 :`B` 1.0 :`A` 1.0)))
          (:`NewEnumerator3`
            (`KismetSystemLibrary.PrintString` "GHOST" true true (struct :`G` 0.078467 :`B` 1.0 :`A` 1.0)))
          (:`NewEnumerator4`
            (`KismetSystemLibrary.PrintString` "WEREWOLF" true true (struct :`G` 0.078467 :`B` 1.0 :`A` 1.0))))))))

(event `/Game/_Game/Blueprint/Core/I_Reaction.StopReact`
  (params (IdName :type Name))
  (`parent.StopReact` IdName)
  (if (not (`self.Moving`))
    (bind _returnvalue (`|GetDataTableRow` "/Game/_Game/Blueprint/NPC/DT_Npc.DT_Npc" IdName)
      (:`then`
        (switch `/Game/_Game/Blueprint/NPC/E_NPCTypes` (`.Types_24_DFB46F504CB588E60C2E12848E012112` (break `/Game/_Game/Blueprint/NPC/FCreatureStruct` _returnvalue))
          (:`NewEnumerator0`
            (`KismetSystemLibrary.PrintString` "HUMAN" true true (struct :`G` 0.078467 :`B` 1.0 :`A` 1.0)))
          (:`NewEnumerator1`
            (`KismetSystemLibrary.PrintString` "DEMON" true true (struct :`G` 0.078467 :`B` 1.0 :`A` 1.0)))
          (:`NewEnumerator2`
            (`KismetSystemLibrary.PrintString` "WITCH" true true (struct :`G` 0.078467 :`B` 1.0 :`A` 1.0)))
          (:`NewEnumerator3`
            (`KismetSystemLibrary.PrintString` "GHOST" true true (struct :`G` 0.078467 :`B` 1.0 :`A` 1.0)))
          (:`NewEnumerator4`
            (`KismetSystemLibrary.PrintString` "WEREWOLF" true true (struct :`G` 0.078467 :`B` 1.0 :`A` 1.0))))))))

(fn `UserConstructionScript`
  (`parent.UserConstructionScript`))